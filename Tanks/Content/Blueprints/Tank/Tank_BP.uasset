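; Tank_BP is a tank Blueprint that lets player input rotate its aiming camera.
; The AimAzimuth axis yaws the AzimuthGimble and AimElevation pitches the SpringArm, separating horizontal and vertical rotation across two components.
; Each local rotation is scaled by world delta seconds and its own speed variable for frame-rate independence, and the construction script is empty.
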(event Input|AxisEvents|InputAxisAimAzimuth
  (params (AxisValue :type Float%20%28single-precision%29))
  ;[1 1 1] Camera input binding
  (Transformation|AddLocalRotation (Variables|Default|GetAzimuthGimble) (Math|Rotator|MakeRotator 0.0 0.0 (* AxisValue (Utilities|Time|GetWorldDeltaSeconds) (Variables|Default|GetAzimuth%20Speed))) false false))

(event Input|AxisEvents|InputAxisAimElevation
  (params (AxisValue :type Float%20%28single-precision%29))
  ;[1 1 1] Camera input binding
  (Transformation|AddLocalRotation (Variables|Default|GetSpringArm) (Math|Rotator|MakeRotator 0.0 (* AxisValue (Utilities|Time|GetWorldDeltaSeconds) (Variables|Default|GetElevation%20Speed)) 0.0) false false))

(fn ConstructionScript)